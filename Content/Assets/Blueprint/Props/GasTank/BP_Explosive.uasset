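; Gas tank prop explosion actor that detonates as soon as it begins play, with sound, Chaos destruction and lethal damage.
; It spawns a short-lived, scaled master field with a radial force to break nearby destructibles.
; A loop of randomly sized sphere traces at random, positive-only offsets from its location applies massive damage to hit pawns, dynamic objects and physics bodies.
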(event EventBeginPlay
  (Audio|PlaySoundatLocation "/Game/StarterContent/Audio/Explosion_Cue.Explosion_Cue" (Transformation|GetActorLocation) "0, 0, 0" 1.0 1.0 0.0 "/Game/Assets/Audio/Attenuation/SA_High.SA_High" 0 0 0)
  (CallFunction|CreateChaosDestruction (Transformation|GetActorLocation) 6.0)
  (for _index (range 0 40)
    (bind (_outhit _returnvalue) (Collision|SphereTraceForObjects (+ (Transformation|GetActorLocation) (Math|Vector|MakeVector (Math|Conversions|ToFloat(Integer) (+ _index (Math|Random|RandomInteger 150))) (Math|Conversions|ToFloat(Integer) (+ _index (Math|Random|RandomInteger 250))) (Math|Conversions|ToFloat(Integer) (+ _index (Math|Random|RandomInteger 80))))) (+ (Transformation|GetActorLocation) (Math|Vector|MakeVector (Math|Conversions|ToFloat(Integer) (+ _index (Math|Random|RandomInteger 150))) (Math|Conversions|ToFloat(Integer) (+ _index (Math|Random|RandomInteger 250))) (Math|Conversions|ToFloat(Integer) (+ _index (Math|Random|RandomInteger 80))))) (Math|Random|RandomFloatinRange 2e+01 2.5e+02) (Utilities|Array|MakeArray "ObjectTypeQuery3" "ObjectTypeQuery2" "ObjectTypeQuery4") true 0 "None"))
    (if _returnvalue
      (Game|Damage|ApplyDamage (.HitActor (Collision|BreakHitResult _outhit)) 9999.0 0 self))))

(fn ConstructionScript)

(fn CreateChaosDestruction
  (params (Spawn%20Transform%20Location :type Vector) (Size :type Float%20%28double-precision%29))
  (bind _returnvalue (Game|SpawnActorfromClass "/Game/Assets/Blueprint/Chaos/FS_MasterField_Custom.FS_MasterField_Custom_C" (Math|Transform|MakeTransform Spawn%20Transform%20Location "0, 0, 0" (Math|Vector|MakeVector Size Size Size)) "AlwaysSpawn" "MultiplyWithRoot" 0 0))
  (Actor|SetLifeSpan _returnvalue 0.5)
  (Variables|/Game/Assets/Blueprint/Chaos/FS_MasterField_Custom.FS_MasterField_Custom_C|SetActivationType _returnvalue "NewEnumerator4")
  (Variables|/Game/Assets/Blueprint/Chaos/FS_MasterField_Custom.FS_MasterField_Custom_C|SetFieldLifespan _returnvalue 0.1)
  (Variables|/Game/Assets/Blueprint/Chaos/FS_MasterField_Custom.FS_MasterField_Custom_C|SetRadial%20Magnitude _returnvalue 1e+03)
  (Default|CETrigger _returnvalue))