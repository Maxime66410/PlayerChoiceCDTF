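; BP_Goo is a destructible goo prop that takes damage and breaks down when its health runs out.
; Any damage is rounded and subtracted from Health; at zero it flags death and, once only, enables physics on the Goo component with a sound.
; A five-second timer is then set, apparently leading to the final event that spawns a goo explosion effect, plays an impact sound and destroys the actor.
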(event Custom|RemoveHealth
  (params (Damage :type Integer))
  ;[0.02879 1 0.1659] Health Logic
  (if (> (Variables|Default|GetHealth) 0)
    (Variables|Default|SetHealth (- (Variables|Default|GetHealth) Damage))
    (if (<= (Variables|Default|GetHealth) 0)
      (Variables|Default|SetIsDeath true :!label _label)
      (CallFunction|DestroyGoo))
    (else
      (goto _label))))

(event Custom|DestroyGoo
  ;[1 0.7892 0] Destroy Goo
  (if (Variables|Default|GetIsDeath)
    (Utilities|FlowControl|DoOnce false
      (:Completed
        (Physics|SetSimulatePhysics (Variables|Default|GetGoo) true)
        (Audio|PlaySoundatLocation "/Game/Assets/Audio/SFX/GasTank/Goo/SC_rock_Cue.SC_rock_Cue" (Transformation|GetActorLocation) "0, 0, 0" 1.0 1.0 0.0 "/Game/Assets/Audio/Attenuation/SA_Medium.SA_Medium" 0 0 0)
        (Utilities|Time|SetTimerbyEvent (EventDispatchers|CreateEvent :!event Custom|DestroyGooDef) 5.0)))))

(event Custom|DestroyGooDef
  ;[0.7857 0 1] Destroy Goo (DestroyActor)
  (Niagara|SpawnSystematLocation "/Game/Assets/Effects/P_Explosion_Goo.P_Explosion_Goo" (Transformation|GetActorLocation))
  (Audio|PlaySoundatLocation "/Game/Assets/Audio/SFX/Physics/Concrete/SC_concrete_impact_hard.SC_concrete_impact_hard" (Transformation|GetActorLocation) "0, 0, 0" 1.0 1.0 0.0 "/Game/Assets/Audio/Attenuation/SA_Medium.SA_Medium" 0 0 0)
  (Actor|DestroyActor))

(event Game|Damage|EventAnyDamage
  (params (Damage :type Float%20%28single-precision%29) (DamageType :type Damage%20Type%20Object%20Reference) (InstigatedBy :type Controller%20Object%20Reference) (DamageCauser :type Actor%20Object%20Reference))
  ;[1 0.228 0.2081] Get Any Damage
  (CallFunction|RemoveHealth (Math|Float|Round Damage)))

(fn ConstructionScript)