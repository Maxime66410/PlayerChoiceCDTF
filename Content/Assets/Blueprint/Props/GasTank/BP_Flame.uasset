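; Gas tank flame actor that spawns a fire explosion with sound and a short-lived Chaos master field for radial destruction.
; A looping one-second timer appears to drive GetDamage, which fires randomized sphere traces around the actor and applies light damage to hit pawns, dynamic objects and physics bodies.
; The traces still draw one-frame debug shapes.
; When its particle system finishes, the actor clears the timer and destroys itself.
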(event OnSystemFinished(ParticleSystem)
  (params (PSystem :type Particle%20System%20Component%20Object%20Reference))
  ;[0.04519 0.02956 0.02843] Destroy Effect
  (Utilities|Time|ClearandInvalidateTimerbyHandle (Variables|Default|GetEvent_GetDamage))
  (Actor|DestroyActor))

(event Custom|GetDamage
  ;[0.02315 0.0356 0.02217] Get Damage
  (for _index (range 0 10)
    (bind (_outhit _returnvalue) (Collision|SphereTraceForObjects (+ (Transformation|GetActorLocation) (Math|Vector|MakeVector (Math|Conversions|ToFloat(Integer) (+ _index (Math|Random|RandomIntegerinRange -150 150))) (Math|Conversions|ToFloat(Integer) (+ _index (Math|Random|RandomIntegerinRange -150 150))) (Math|Conversions|ToFloat(Integer) (+ _index (Math|Random|RandomIntegerinRange -80 80))))) (+ (Transformation|GetActorLocation) (Math|Vector|MakeVector (Math|Conversions|ToFloat(Integer) (+ _index (Math|Random|RandomIntegerinRange -150 150))) (Math|Conversions|ToFloat(Integer) (+ _index (Math|Random|RandomIntegerinRange -150 150))) (Math|Conversions|ToFloat(Integer) (+ _index (Math|Random|RandomIntegerinRange -80 80))))) (Math|Random|RandomFloatinRange 2e+01 1.5e+02) (Utilities|Array|MakeArray "ObjectTypeQuery3" "ObjectTypeQuery2" "ObjectTypeQuery4") true 0 "ForOneFrame"))
    (if _returnvalue
      (Game|Damage|ApplyDamage (.HitActor (Collision|BreakHitResult _outhit)) 1.0 0 self))))

(event EventBeginPlay
  ;[0.04971 0.1022 0.147] Begin play
  (Effects|SpawnEmitteratLocation "/Game/Assets/Effects/M5VFXVOL2/Particles/Explosion/Fire_Exp_00.Fire_Exp_00" (Transformation|GetActorLocation))
  (Audio|PlaySoundatLocation "/Game/StarterContent/Audio/Explosion_Cue.Explosion_Cue" (Transformation|GetActorLocation) "0, 0, 0" 1.0 1.0 0.0 "/Game/Assets/Audio/Attenuation/SA_High.SA_High" 0 0 0)
  (CallFunction|CreateChaosDestruction (Transformation|GetActorLocation) 4.0)
  (bind _returnvalue (Utilities|Time|SetTimerbyEvent (EventDispatchers|CreateEvent :!event Custom|GetDamage) 1.0 true))
  (Variables|Default|SetEvent_GetDamage _returnvalue))

(fn ConstructionScript)

(fn CreateChaosDestruction
  (params (Spawn%20Transform%20Location :type Vector) (Size :type Float%20%28double-precision%29))
  (bind _returnvalue (Game|SpawnActorfromClass "/Game/Assets/Blueprint/Chaos/FS_MasterField_Custom.FS_MasterField_Custom_C" (Math|Transform|MakeTransform Spawn%20Transform%20Location "0, 0, 0" (Math|Vector|MakeVector Size Size Size)) "AlwaysSpawn" "MultiplyWithRoot" 0 0))
  (Actor|SetLifeSpan _returnvalue 0.5)
  (Variables|/Game/Assets/Blueprint/Chaos/FS_MasterField_Custom.FS_MasterField_Custom_C|SetActivationType _returnvalue "NewEnumerator4")
  (Variables|/Game/Assets/Blueprint/Chaos/FS_MasterField_Custom.FS_MasterField_Custom_C|SetFieldLifespan _returnvalue 0.1)
  (Variables|/Game/Assets/Blueprint/Chaos/FS_MasterField_Custom.FS_MasterField_Custom_C|SetRadial%20Magnitude _returnvalue 1e+03)
  (Default|CETrigger _returnvalue))