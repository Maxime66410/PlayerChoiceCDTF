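; Goo spawner among the gas tank props that lays out rows of BP_Goo actors around itself on BeginPlay.
; GenerateGooDirection runs once per quadrant, stepping along world X from points offset above and below the actor to spawn up to five goo each.
; Before each spawn a visibility line trace runs along the actor's forward or backward axis, and the first hit ends that row.
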(event EventBeginPlay
  (CallFunction|GenerateGooDirection "NewEnumerator0")
  (CallFunction|GenerateGooDirection "NewEnumerator1")
  (CallFunction|GenerateGooDirection "NewEnumerator2")
  (CallFunction|GenerateGooDirection "NewEnumerator3"))

(fn ConstructionScript)

(fn GenerateGooDirection
  (params (Direection :type EGooDirection%20Enum :default "NewEnumerator0"))
  (LocalVariables|SetActorLocation (Transformation|GetActorLocation))
  (LocalVariables|SetActorRotation (Transformation|GetActorRotation))
  (switch Utilities|FlowControl|Switch|SwitchonEGooDirection Direection
    (:NewEnumerator0
      (bind _index (Utilities|FlowControl|ForLoopwithBreak 0 4 :!label _label)
        (:LoopBody
          (bind _output_get (LocalVariables|SetActorLocationMove (+ (+ (LocalVariables|GetActorLocation) "0.000000,0.000000,70.000000") (* _index "100.000000,0.000000,0.000000"))))
          (bind (_outhit _returnvalue) (Collision|LineTraceByChannel _output_get (+ (+ (+ (LocalVariables|GetActorLocation) "0.000000,0.000000,70.000000") (* _index "100.000000,0.000000,0.000000")) (* (Math|Vector|GetForwardVector (LocalVariables|GetActorRotation)) -2e+02)) "TraceTypeQuery1" true 0 "ForOneFrame"))
          (if _returnvalue
            (goto _label Break)
            (else
              (bind _returnvalue_2 (Game|SpawnActorfromClass "/Game/Assets/Blueprint/Props/GasTank/BP_Goo.BP_Goo_C" (Math|Transform|MakeTransform (LocalVariables|GetActorLocationMove) (LocalVariables|GetActorRotation) "1.000000,1.000000,1.000000") "AlwaysSpawn" "MultiplyWithRoot" 0 0))
              (LocalVariables|SetActorRotation (Transformation|GetActorRotation _returnvalue_2)))))))
    (:NewEnumerator1
      (bind _index_2 (Utilities|FlowControl|ForLoopwithBreak 0 4 :!label _label_2)
        (:LoopBody
          (bind _output_get_2 (LocalVariables|SetActorLocationMove (+ (+ (LocalVariables|GetActorLocation) "0.000000,0.000000,-70.000000") (* _index_2 "100.000000,0.000000,0.000000"))))
          (bind (_outhit_2 _returnvalue_3) (Collision|LineTraceByChannel _output_get_2 (+ (+ (+ (LocalVariables|GetActorLocation) "0.000000,0.000000,-70.000000") (* _index_2 "100.000000,0.000000,0.000000")) (* (Math|Vector|GetForwardVector (LocalVariables|GetActorRotation)) -2e+02)) "TraceTypeQuery1" true 0 "ForOneFrame"))
          (if _returnvalue_3
            (goto _label_2 Break)
            (else
              (bind _returnvalue_4 (Game|SpawnActorfromClass "/Game/Assets/Blueprint/Props/GasTank/BP_Goo.BP_Goo_C" (Math|Transform|MakeTransform (LocalVariables|GetActorLocationMove) (LocalVariables|GetActorRotation) "1.000000,1.000000,1.000000") "AlwaysSpawn" "MultiplyWithRoot" 0 0))
              (LocalVariables|SetActorRotation (Transformation|GetActorRotation _returnvalue_4)))))))
    (:NewEnumerator2
      (bind _index_3 (Utilities|FlowControl|ForLoopwithBreak 0 4 :!label _label_3)
        (:LoopBody
          (bind _output_get_3 (LocalVariables|SetActorLocationMove (+ (+ (LocalVariables|GetActorLocation) "0.000000,0.000000,70.000000") (* _index_3 "-100.000000,0.000000,0.000000"))))
          (bind (_outhit_3 _returnvalue_5) (Collision|LineTraceByChannel _output_get_3 (+ (+ (+ (LocalVariables|GetActorLocation) "0.000000,0.000000,70.000000") (* _index_3 "-100.000000,0.000000,0.000000")) (* (Math|Vector|GetForwardVector (LocalVariables|GetActorRotation)) 2e+02)) "TraceTypeQuery1" true 0 "ForOneFrame"))
          (if _returnvalue_5
            (goto _label_3 Break)
            (else
              (bind _returnvalue_6 (Game|SpawnActorfromClass "/Game/Assets/Blueprint/Props/GasTank/BP_Goo.BP_Goo_C" (Math|Transform|MakeTransform (LocalVariables|GetActorLocationMove) (LocalVariables|GetActorRotation) "1.000000,1.000000,1.000000") "AlwaysSpawn" "MultiplyWithRoot" 0 0))
              (LocalVariables|SetActorRotation (Transformation|GetActorRotation _returnvalue_6)))))))
    (:NewEnumerator3
      (bind _index_4 (Utilities|FlowControl|ForLoopwithBreak 0 4 :!label _label_4)
        (:LoopBody
          (bind _output_get_4 (LocalVariables|SetActorLocationMove (+ (+ (LocalVariables|GetActorLocation) "0.000000,0.000000,-70.000000") (* _index_4 "-100.000000,0.000000,0.000000"))))
          (bind (_outhit_4 _returnvalue_7) (Collision|LineTraceByChannel _output_get_4 (+ (+ (+ (LocalVariables|GetActorLocation) "0.000000,0.000000,-70.000000") (* _index_4 "-100.000000,0.000000,0.000000")) (* (Math|Vector|GetForwardVector (LocalVariables|GetActorRotation)) 2e+02)) "TraceTypeQuery1" true 0 "ForOneFrame"))
          (if _returnvalue_7
            (goto _label_4 Break)
            (else
              (bind _returnvalue_8 (Game|SpawnActorfromClass "/Game/Assets/Blueprint/Props/GasTank/BP_Goo.BP_Goo_C" (Math|Transform|MakeTransform (LocalVariables|GetActorLocationMove) (LocalVariables|GetActorRotation) "1.000000,1.000000,1.000000") "AlwaysSpawn" "MultiplyWithRoot" 0 0))
              (LocalVariables|SetActorRotation (Transformation|GetActorRotation _returnvalue_8)))))))))