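; Toxic cloud hazard, filed with the gas tank prop, that deals periodic damage until its particle effect finishes.
; A looping one-second timer set on BeginPlay drives bursts of randomly placed, randomly sized sphere traces around the actor.
; Each hit on a pawn, dynamic or physics object applies minor damage, and debug drawing is left on.
; When the particle system finishes, it clears the timer and destroys the actor.
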(event OnSystemFinished(ParticleSystem)
  (params (PSystem :type Particle%20System%20Component%20Object%20Reference))
  ;[0.04519 0.02956 0.02843] Destroy Effect
  (Utilities|Time|ClearandInvalidateTimerbyHandle (Variables|Default|GetEvent_GetDamage))
  (Actor|DestroyActor))

(event Custom|GetDamage
  ;[0.02315 0.0356 0.02217] Get Damage
  (for _index (range 0 10)
    (bind (_outhit _returnvalue) (Collision|SphereTraceForObjects (+ (Transformation|GetActorLocation) (Math|Vector|MakeVector (Math|Conversions|ToFloat(Integer) (+ _index (Math|Random|RandomIntegerinRange -150 150))) (Math|Conversions|ToFloat(Integer) (+ _index (Math|Random|RandomIntegerinRange -250 250))) (Math|Conversions|ToFloat(Integer) (+ _index (Math|Random|RandomIntegerinRange -80 80))))) (+ (Transformation|GetActorLocation) (Math|Vector|MakeVector (Math|Conversions|ToFloat(Integer) (+ _index (Math|Random|RandomIntegerinRange -150 150))) (Math|Conversions|ToFloat(Integer) (+ _index (Math|Random|RandomIntegerinRange -250 250))) (Math|Conversions|ToFloat(Integer) (+ _index (Math|Random|RandomIntegerinRange -80 80))))) (Math|Random|RandomFloatinRange 2e+01 2.5e+02) (Utilities|Array|MakeArray "ObjectTypeQuery3" "ObjectTypeQuery2" "ObjectTypeQuery4") true 0 "ForOneFrame"))
    (if _returnvalue
      (Game|Damage|ApplyDamage (.HitActor (Collision|BreakHitResult _outhit)) 1.0 0 self))))

(event EventBeginPlay
  ;[0.04971 0.1022 0.147] Begin play
  (bind _returnvalue (Utilities|Time|SetTimerbyEvent (EventDispatchers|CreateEvent :!event Custom|GetDamage) 1.0 true))
  (Variables|Default|SetEvent_GetDamage _returnvalue))

(fn ConstructionScript)