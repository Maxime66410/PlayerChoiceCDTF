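; Master physics prop that the player can grab, drop and throw, with a prop type selecting mesh, health, impact sounds and destruction effect.
; While held, physics and collision are off and Tick interpolates it to the player's hold point.
; Hits play velocity-tiered sounds and self-damage, throttled by timer-reset DoOnce gates, with optional lethal damage after throws.
; Damage destroys it with an effect, immediately or at zero health when health is enabled.
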(event OnComponentHit(PropsModels)
  (params (HitComponent :type Primitive%20Component%20Object%20Reference) (OtherActor :type Actor%20Object%20Reference) (OtherComp :type Primitive%20Component%20Object%20Reference) (NormalImpulse :type Vector :default "0, 0, 0") (Hit :type Hit%20Result%20Structure%20%28by%20ref%29))
  (bind _self self)
  (bind _self_2 self)
  (bind _plrref (Variables|Target|GetPlrRef))
  (bind _returnvalue (Transformation|GetActorRotation _plrref))
  (bind _returnvalue_2 (Math|Vector|GetForwardVector _returnvalue))
  (bind _returnvalue_3 (* _returnvalue_2 2e+02))
  (bind (_x _y) (Math|Vector|BreakVector _returnvalue_3))
  ;[0.4134 0 1] Hit Component
  (Utilities|Casting|CastToBP_Player OtherActor
    (:then
      ;;[1 0.3729 0.343] Is Grabbed Component Hit
      (Variables|Target|SetIsPlayerHit? true))
    (:CastFailed
      (if (and (Variables|Target|GetIsGrabbed) (not (Variables|Target|GetIsGrabbedLaunch?)))
        (SETTER|SetPhysics false)
        (SETTER|SetCollisionsChannels "ECC_Pawn" "ECR_Ignore")
        (Transformation|SetActorRotation (Math|Rotator|MakeRotator 0.0 0.0 (.yaw (Transformation|GetActorRotation))) true)
        (Transformation|SetActorLocation (+ (+ (.ImpactPoint (Collision|BreakHitResult Hit)) "0.000000,0.000000,80.000000") (Math|Vector|MakeVector _x _y 0.0)) false true)
        (Variables|Target|SetIsGrabbed false)
        (SETTER|SetCollisionsChannels "ECC_Pawn" "ECR_Block")
        (Physics|SetPhysicsLinearVelocity (Variables|Default|GetPropsModels) "0, 0, 0" false "None")
        (SETTER|SetPhysics true)
        (elif (Variables|Target|GetIsGrabbedLaunch?)
          (if (Variables|ProfileProps|GetDamageByLaunch)
            ;;[1 0.8465 0] Set Ultra Damage Because player Launch Object
            (Audio|PlaySoundatLocation (Utilities|GetLoudHit) (Transformation|GetActorLocation) "0, 0, 0" 1.0 1.0 0.0 "/Game/Assets/Audio/Attenuation/SA_Low.SA_Low" 0 0 0)
            (Game|Damage|ApplyDamage _self 99999.0 0 _self)
            (else
              ;;[0.1941 1 0] Set Damage by Hit
              (if (> (GETTER|GetVelocityActor) 3e+02) :!label _label
                (if (> (GETTER|GetVelocityActor) 1e+03)
                  (Utilities|FlowControl|DoOnce false
                    (:Completed
                      ;;;[1 0.1118 0] Play Sound LOUD and Get LOUD Damage with 1000 Velocity
                      (if (not (Variables|Target|GetIsPlayerHit?))
                        (Audio|PlaySoundatLocation (Utilities|GetLoudHit) (Transformation|GetActorLocation) "0, 0, 0" 1.0 1.0 0.0 "/Game/Assets/Audio/Attenuation/SA_Low.SA_Low" 0 0 0)
                        (Game|Damage|ApplyDamage _self_2 15.0 0 _self_2)
                        (else
                          (Variables|Target|SetIsPlayerHit? false)))
                      (CallFunction|StartResetOnceHit)))
                  (else
                    (Utilities|FlowControl|DoOnce false
                      (:Completed
                        ;;;[0 1 0.8703] Play Sound Normal and Get Little Damage with 300 Velocity
                        (if (not (Variables|Target|GetIsPlayerHit?))
                          (Audio|PlaySoundatLocation (Utilities|GetSoftHit) (Transformation|GetActorLocation) "0, 0, 0" 1.0 1.0 0.0 "/Game/Assets/Audio/Attenuation/SA_Low.SA_Low" 0 0 0)
                          (Game|Damage|ApplyDamage _self_2 5.0 0 _self_2)
                          (else
                            (Variables|Target|SetIsPlayerHit? false)))
                        (CallFunction|StartResetOnceHit)))))
                (else
                  ;;;[0.25 0.02416 1] Play Sound just for details
                  (if (> (GETTER|GetVelocityActor) 2e+02)
                    (if (not (Variables|Target|GetIsPlayerHit?))
                      (Utilities|FlowControl|DoOnce false
                        (:Completed
                          (Audio|PlaySoundatLocation (Utilities|GetSoftHit) (Transformation|GetActorLocation) "0, 0, 0" 1.0 1.0 0.0 "/Game/Assets/Audio/Attenuation/SA_Low.SA_Low" 0 0 0)))
                      (else
                        (Variables|Target|SetIsPlayerHit? false)))
                    (CallFunction|StartResetOnceHit)
                    (else
                      (Variables|Target|SetIsPlayerHit? false)))))))
          (else
            (goto _label)))))))

(event Custom|DEBUG_ShowVelocity
  (bind _propsmodels (Variables|Default|GetPropsModels))
  (bind _returnvalue (Transformation|GetComponentVelocity _propsmodels))
  (Development|PrintText (Utilities|Text|FormatText "NORMAL : {A} 
SQR : {B}" (Math|Vector|VectorLength _returnvalue) (Math|Vector|VectorLengthSquared _returnvalue)) true true "(R=0.000000,G=0.660000,B=1.000000,A=1.000000)" 0.005))

(event Custom|AutoResetCollision
  ;[0.9915 1 0.1511] Auto Reset Collisions
  (Variables|Target|SetIsGrabbed false)
  (SETTER|SetCollisionsChannels "ECC_Pawn" "ECR_Block"))

(event Custom|ResetDoOnceHit
  (bind _self self)
  ;[0.4134 0 1] Hit Component
  ;;[0.1941 1 0] Set Damage by Hit
  ;;;[1 0 0.901] Reset Take Damage
  (Utilities|FlowControl|Sequence
    (:then_0
      (Utilities|FlowControl|DoOnce false) ; enters at Reset
    )
    (:then_1
      (Utilities|FlowControl|DoOnce false) ; enters at Reset
    )
    (:then_2
      ;;;[0.25 0.02416 1] Play Sound just for details
      (Utilities|FlowControl|DoOnce false) ; enters at Reset
    )))

(event Custom|StartResetOnceHit
  ;[0.4134 0 1] Hit Component
  ;;[0.06965 0 1] Start Reset Once Hit
  (Utilities|Time|SetTimerbyEvent (EventDispatchers|CreateEvent :!event Custom|ResetDoOnceHit) 1.0))

(event EventLaunchObject
  (params (Plr :type BP%20Player%20Object%20Reference))
  ;[0.1356 0.05951 0.2086] Throw Actor
  (Utilities|FlowControl|Sequence
    (:then_0
      (Variables|Target|SetIsPickup? false)
      (Default|SetActorAttachGrab Plr)
      (Default|SetIsObjectPickup Plr false)
      (Variables|Target|SetIsGrabbedLaunch? true))
    (:then_1
      (Actor|Tick|SetActorTickEnabled false))
    (:then_2
      (SETTER|SetCollisions "QueryAndPhysics")
      (SETTER|SetPhysics true))
    (:then_3
      (Utilities|Time|SetTimerbyEvent (EventDispatchers|CreateEvent :!event Custom|AutoResetCollision) 0.005))
    (:then_4
      (Physics|SetPhysicsLinearVelocity (Variables|Default|GetPropsModels) (* (Math|Vector|GetForwardVector (Variables|/Game/Assets/Blueprint/Player/BP_Player.BP_Player_C|GetFPSCamera Plr)) 1.2e+03) false "None"))))

(event EventDropObject
  (params (Plr :type BP%20Player%20Object%20Reference))
  ;[0.001821 0.04971 0.2462] Drop BPI
  (Variables|Target|SetIsPickup? false)
  (Default|SetActorAttachGrab Plr)
  (Default|SetIsObjectPickup Plr false)
  (Utilities|FlowControl|Sequence
    (:then_0
      (Actor|Tick|SetActorTickEnabled false))
    (:then_1
      (SETTER|SetCollisions "QueryAndPhysics")
      (SETTER|SetPhysics true))
    (:then_2
      (Utilities|Time|SetTimerbyEvent (EventDispatchers|CreateEvent :!event Custom|AutoResetCollision) 0.005))))

(event EventGrabObject
  (params (Plr :type BP%20Player%20Object%20Reference))
  ;[0.2271 0.3215 1] Grab BPI
  (bind _output_get (Variables|Target|SetPlrRef Plr))
  (Variables|Target|SetComponentToTarget (Variables|/Game/Assets/Blueprint/Player/BP_Player.BP_Player_C|GetObjectPos _output_get))
  (Default|SetActorAttachGrab (Variables|Target|GetPlrRef) self)
  (Utilities|FlowControl|Sequence
    (:then_0
      (Variables|Target|SetIsPickup? true)
      (Variables|Target|SetIsGrabbed true))
    (:then_1
      (SETTER|SetPhysics false))
    (:then_2
      (SETTER|SetCollisions "NoCollision")
      (SETTER|SetCollisionsChannels "ECC_Pawn" "ECR_Ignore"))
    (:then_3
      (Actor|Tick|SetActorTickEnabled true))))

(event EventTick
  (params (DeltaSeconds :type Float%20%28single-precision%29))
  ;[0.07292 0.001139 0.001139] TICK
  (Variables|Tick|SetDelta%20Seconds DeltaSeconds)
  (Tick|FollowObject))

(event Game|Damage|EventAnyDamage
  (params (Damage :type Float%20%28single-precision%29) (DamageType :type Damage%20Type%20Object%20Reference) (InstigatedBy :type Controller%20Object%20Reference) (DamageCauser :type Actor%20Object%20Reference))
  ;[0.04667 0.2086 0.15] Get Any Damage
  (if (Variables|ProfileProps|GetIsHealth?)
    (if (> (Variables|ProfileProps|GetHealth) 0)
      (Variables|ProfileProps|SetHealth (- (Variables|ProfileProps|GetHealth) (Math|Float|Round Damage)))
      (if (<= (Variables|ProfileProps|GetHealth) 0)
        (CallFunction|DestroyActorbyHit))
      (else
        (CallFunction|DestroyActorbyHit)))
    (else
      (CallFunction|DestroyActorbyHit))))

(event EventBeginPlay
  (Class|PrimitiveComponent|SetAllMassScale (Variables|Default|GetPropsModels) (Variables|ProfileProps|GetWeigh)))

(fn ConstructionScript
  (Components|StaticMesh|SetStaticMesh (Variables|Default|GetPropsModels) (Utilities|GetMesh))
  (Physics|SetSimulatePhysics (Variables|Default|GetPropsModels) (Variables|ProfileProps|GetIsPhysics?))
  (if (== (Variables|ProfileProps|GetHealth) 0)
    (Variables|ProfileProps|SetHealth (Utilities|GetHealth))))

(fn FollowObject
  (bind _componenttotarget (Variables|Target|GetComponentToTarget))
  (Variables|Target|GetPlrRef
    (:then
      (Variables|Target|GetComponentToTarget
        (:then
          (if (Variables|Target|GetIsPickup?)
            (LocalVariables|SetCompLoc (Transformation|GetWorldLocation _componenttotarget))
            (LocalVariables|SetCompRot (Transformation|GetWorldRotation _componenttotarget))
            (Transformation|SetActorLocation (Math|Interpolation|VInterpTo (Transformation|GetActorLocation) (LocalVariables|GetCompLoc) (Variables|Tick|GetDelta%20Seconds) 4e+01) false false)
            (Transformation|SetActorRotation (Math|Interpolation|RInterpTo (Transformation|GetActorRotation) (LocalVariables|GetCompRot) (Variables|Tick|GetDelta%20Seconds) 2e+01))))
        (:else)))
    (:else)))

(fn SetCollisions
  (params (NewType :type ECollisionEnabled%20Enum :default "NoCollision"))
  (Collision|SetCollisionEnabled (Variables|Default|GetPropsModels) NewType))

(fn SetPhysics
  (params (bSimulate :type Boolean))
  (Physics|SetSimulatePhysics (Variables|Default|GetPropsModels) bSimulate))

(fn SetCollisionsChannels
  (params (Channel :type ECollisionChannel%20Enum :default "ECC_WorldStatic") (NewResponse :type ECollisionResponse%20Enum :default "ECR_Ignore"))
  (Collision|SetCollisionResponsetoChannel (Variables|Default|GetPropsModels) Channel NewResponse))

(fn DestroyActorbyHit
  (Effects|SpawnEmitteratLocation (Utilities|GetEffecttoDestroy) (Transformation|GetActorLocation))
  (Actor|DestroyActor))

(fn GetVelocityActor
  (return (Math|Vector|VectorLength (Transformation|GetComponentVelocity (Variables|Default|GetPropsModels)))))