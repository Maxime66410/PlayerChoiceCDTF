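; BP_Stimpak is a health pickup that heals the player when they walk into its box trigger.
; On overlap it casts to BP_Player and, only if health is below the full threshold, adds health, plays a medkit sound and destroys itself.
; Tick spins the stimpak model and its sign component by a fixed step each frame, so the rotation speed depends on frame rate.
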(event OnComponentBeginOverlap(Box)
  (params (OverlappedComponent :type Primitive%20Component%20Object%20Reference) (OtherActor :type Actor%20Object%20Reference) (OtherComp :type Primitive%20Component%20Object%20Reference) (OtherBodyIndex :type Integer) (bFromSweep :type Boolean) (SweepResult :type Hit%20Result%20Structure%20%28by%20ref%29))
  (bind _asbp_player (Utilities|Casting|CastToBP_Player OtherActor))
  (if (not (>= (Default|GetHealth _asbp_player) 100))
    (Default|AddHealth _asbp_player 25)
    (Audio|PlaySound2D "/Game/Assets/Audio/SFX/UI/SW_Half_Life_Medkit_Sound_Effect.SW_Half_Life_Medkit_Sound_Effect" 0.5 1.0 0.0 0 0)
    (Actor|DestroyActor)))

(event EventTick
  (params (DeltaSeconds :type Float%20%28single-precision%29))
  (Transformation|AddLocalRotation (Variables|Default|GetStimpakModel) "0.500000,0.000000,0.000000" false false)
  (Transformation|AddLocalRotation (Variables|Default|GetSigne) "0.000000,0.300000,0.000000" false false))

(fn ConstructionScript)