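; Physics gas tank prop the player can grab, drop or throw, with GasType choosing mesh and material.
; While held, it interpolates to the player's hold point on Tick; sphere overlaps turn throws into drops.
; Hard impacts, scaled by speed, play sounds, self-damage and spawn Chaos fields.
; Any damage destroys it with an effect, spawning an explosion or goo actor for those types; other types have no spawn class.
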(event OnComponentBeginOverlap(Sphere)
  (params (OverlappedComponent :type Primitive%20Component%20Object%20Reference) (OtherActor :type Actor%20Object%20Reference) (OtherComp :type Primitive%20Component%20Object%20Reference) (OtherBodyIndex :type Integer) (bFromSweep :type Boolean) (SweepResult :type Hit%20Result%20Structure%20%28by%20ref%29))
  ;[0.006512 0.05951 0.1022] Overlap Collision System To Place Props
  (if (not (Utilities|Array|ContainsItem (Variables|OnTrigger|GetGetActorHit) OtherActor))
    (Utilities|Array|Add (Variables|OnTrigger|GetGetActorHit) OtherActor)
    (bind _plrref (Variables|Target|GetPlrRef)
      (:then
        (Default|SetEffectGrabColor _plrref true)
        (Variables|OnTrigger|SetIsInCollision true))
      (:else))))

(event OnComponentEndOverlap(Sphere)
  (params (OverlappedComponent :type Primitive%20Component%20Object%20Reference) (OtherActor :type Actor%20Object%20Reference) (OtherComp :type Primitive%20Component%20Object%20Reference) (OtherBodyIndex :type Integer))
  (bind _getactorhit (Variables|OnTrigger|GetGetActorHit))
  ;[0.006512 0.05951 0.1022] Overlap Collision System To Place Props
  (Utilities|Array|RemoveIndex _getactorhit (Utilities|Array|FindItem _getactorhit OtherActor))
  (if (Utilities|Array|IsEmpty _getactorhit)
    (bind _plrref (Variables|Target|GetPlrRef)
      (:then
        (Default|SetEffectGrabColor _plrref false)
        (Variables|OnTrigger|SetIsInCollision false))
      (:else))))

(event OnComponentHit(GasTank)
  (params (HitComponent :type Primitive%20Component%20Object%20Reference) (OtherActor :type Actor%20Object%20Reference) (OtherComp :type Primitive%20Component%20Object%20Reference) (NormalImpulse :type Vector :default "0, 0, 0") (Hit :type Hit%20Result%20Structure%20%28by%20ref%29))
  (bind _self self)
  (bind _self_2 self)
  (bind _plrref (Variables|Target|GetPlrRef))
  (bind _returnvalue (Transformation|GetActorRotation _plrref))
  (bind _returnvalue_2 (Math|Vector|GetForwardVector _returnvalue))
  (bind _returnvalue_3 (* _returnvalue_2 2e+02))
  (bind (_x _y) (Math|Vector|BreakVector _returnvalue_3))
  ;[0.4134 0 1] Hit Component
  (if (not (Variables|Target|GetIsPickup?))
    (Variables|Default|SetLast%20Impact%20Point (.ImpactPoint (Collision|BreakHitResult Hit)))
    (Utilities|Casting|CastToBP_Player OtherActor
      (:then
        ;;[1 0.3729 0.343] Is Grabbed Component Hit
        (Variables|Target|SetIsPlayerHit? true))
      (:CastFailed
        (if (and (Variables|Target|GetIsGrabbed) (not (Variables|Target|GetIsGrabbedLaunch?)))
          (SETTER|SetPhysics false)
          (SETTER|SetCollisionsChannels "ECC_Pawn" "ECR_Ignore")
          (Transformation|SetActorRotation (Math|Rotator|MakeRotator 0.0 0.0 (.yaw (Transformation|GetActorRotation))) true)
          (Transformation|SetActorLocation (+ (+ (.ImpactPoint (Collision|BreakHitResult Hit)) "0.000000,0.000000,80.000000") (Math|Vector|MakeVector _x _y 0.0)) false true)
          (Variables|Target|SetIsGrabbed false)
          (SETTER|SetCollisionsChannels "ECC_Pawn" "ECR_Block")
          (Physics|SetPhysicsLinearVelocity (Variables|Default|GetGasTank) "0, 0, 0" false "None")
          (SETTER|SetPhysics true)
          (elif (Variables|Target|GetIsGrabbedLaunch?)
            (if (Variables|ProfileTank|GetDamageByLaunch)
              ;;[1 0.8465 0] Set Ultra Damage Because player Launch Object
              (Audio|PlaySoundatLocation (Utilities|GetLoudHit) (Transformation|GetActorLocation) "0, 0, 0" 1.0 1.0 0.0 "/Game/Assets/Audio/Attenuation/SA_Low.SA_Low" 0 0 0)
              (Game|Damage|ApplyDamage _self 99999.0 0 _self)
              (AUTO|CreateChaosDestruction (Variables|Default|GetLast%20Impact%20Point) 0.4)
              (else
                ;;[0.1941 1 0] Set Damage by Hit
                (if (> (GETTER|GetVelocityActor) 3e+02) :!label _label
                  (if (> (GETTER|GetVelocityActor) 1e+03)
                    (Utilities|FlowControl|DoOnce false
                      (:Completed
                        ;;;[1 0.1118 0] Play Sound LOUD and Get LOUD Damage with 1000 Velocity
                        (if (not (Variables|Target|GetIsPlayerHit?))
                          (Audio|PlaySoundatLocation (Utilities|GetLoudHit) (Transformation|GetActorLocation) "0, 0, 0" 1.0 1.0 0.0 "/Game/Assets/Audio/Attenuation/SA_Low.SA_Low" 0 0 0)
                          (Game|Damage|ApplyDamage _self_2 15.0 0 _self_2)
                          (else
                            (Variables|Target|SetIsPlayerHit? false)))
                        (CallFunction|StartResetOnceHit)
                        (AUTO|CreateChaosDestruction (Variables|Default|GetLast%20Impact%20Point) 0.4)))
                    (else
                      (Utilities|FlowControl|DoOnce false
                        (:Completed
                          ;;;[0 1 0.8703] Play Sound Normal and Get Little Damage with 300 Velocity
                          (if (not (Variables|Target|GetIsPlayerHit?))
                            (Audio|PlaySoundatLocation (Utilities|GetSoftHit) (Transformation|GetActorLocation) "0, 0, 0" 1.0 1.0 0.0 "/Game/Assets/Audio/Attenuation/SA_Low.SA_Low" 0 0 0)
                            (Game|Damage|ApplyDamage _self_2 5.0 0 _self_2)
                            (else
                              (Variables|Target|SetIsPlayerHit? false)))
                          (CallFunction|StartResetOnceHit)
                          (AUTO|CreateChaosDestruction (Variables|Default|GetLast%20Impact%20Point) 0.3)))))
                  (else
                    ;;;[0.25 0.02416 1] Play Sound just for details
                    (if (> (GETTER|GetVelocityActor) 2e+02)
                      (if (not (Variables|Target|GetIsPlayerHit?))
                        (Utilities|FlowControl|DoOnce false
                          (:Completed
                            (Audio|PlaySoundatLocation (Utilities|GetSoftHit) (Transformation|GetActorLocation) "0, 0, 0" 1.0 1.0 0.0 "/Game/Assets/Audio/Attenuation/SA_Low.SA_Low" 0 0 0)))
                        (else
                          (Variables|Target|SetIsPlayerHit? false)))
                      (CallFunction|StartResetOnceHit)
                      (else
                        (Variables|Target|SetIsPlayerHit? false)))))))
            (else
              (goto _label))))))))

(event Custom|DEBUG_ShowVelocity
  (bind _gastank (Variables|Default|GetGasTank))
  (bind _returnvalue (Transformation|GetComponentVelocity _gastank))
  (Development|PrintText (Utilities|Text|FormatText "NORMAL : {A} 
SQR : {B}" (Math|Vector|VectorLength _returnvalue) (Math|Vector|VectorLengthSquared _returnvalue)) true true "(R=0.000000,G=0.660000,B=1.000000,A=1.000000)" 0.005))

(event Custom|AutoResetCollision
  ;[0.9915 1 0.1511] Auto Reset Collisions
  (Variables|Target|SetIsGrabbed false)
  (SETTER|SetCollisionsChannels "ECC_Pawn" "ECR_Block"))

(event Custom|ResetDoOnceHit
  (bind _self self)
  ;[0.4134 0 1] Hit Component
  ;;[0.1941 1 0] Set Damage by Hit
  ;;;[1 0 0.901] Reset Take Damage
  (Utilities|FlowControl|Sequence
    (:then_0
      (Utilities|FlowControl|DoOnce false) ; enters at Reset
    )
    (:then_1
      (Utilities|FlowControl|DoOnce false) ; enters at Reset
    )
    (:then_2
      ;;;[0.25 0.02416 1] Play Sound just for details
      (Utilities|FlowControl|DoOnce false) ; enters at Reset
    )))

(event Custom|StartResetOnceHit
  ;[0.4134 0 1] Hit Component
  ;;[0.06965 0 1] Start Reset Once Hit
  (Utilities|Time|SetTimerbyEvent (EventDispatchers|CreateEvent :!event Custom|ResetDoOnceHit) 1.0))

(event Custom|ForceDrop
  (params (Plr :type BP%20Player%20Object%20Reference))
  ;[0.001821 0.04971 0.2462] Drop BPI
  (Variables|Target|SetPlrRef Plr)
  (Variables|Target|SetIsPickup? false)
  (Default|SetActorAttachGrab (Variables|Target|GetPlrRef))
  (Default|SetIsObjectPickup (Variables|Target|GetPlrRef) false)
  (Utilities|FlowControl|Sequence
    (:then_0
      (Actor|Tick|SetActorTickEnabled false))
    (:then_1
      (SETTER|SetCollisions "QueryAndPhysics")
      (SETTER|SetChannels "ECC_WorldDynamic")
      (SETTER|SetPhysics true))
    (:then_2
      (Utilities|Time|SetTimerbyEvent (EventDispatchers|CreateEvent :!event Custom|AutoResetCollision) 0.005)
      (Default|SettoCurrentWeapons (Variables|Target|GetPlrRef))
      (Default|SetEffectGrabObject (Variables|Target|GetPlrRef) true)
      (Default|SetColorPostLine (Variables|Target|GetPlrRef) false))))

(event EventLaunchObject
  (params (Plr :type BP%20Player%20Object%20Reference))
  ;[0.1356 0.05951 0.2086] Throw Actor
  (if (not (Variables|OnTrigger|GetIsInCollision))
    (Utilities|FlowControl|Sequence
      (:then_0
        (Variables|Target|SetIsPickup? false)
        (Default|SetActorAttachGrab Plr)
        (Default|SetIsObjectPickup Plr false)
        (Variables|Target|SetIsGrabbedLaunch? true))
      (:then_1
        (Actor|Tick|SetActorTickEnabled false))
      (:then_2
        (SETTER|SetCollisions "QueryAndPhysics")
        (SETTER|SetChannels "ECC_WorldDynamic")
        (SETTER|SetPhysics true))
      (:then_3
        (Utilities|Time|SetTimerbyEvent (EventDispatchers|CreateEvent :!event Custom|AutoResetCollision) 0.005)
        (Default|SetEffectGrabObject (Variables|Target|GetPlrRef) true)
        (Default|CallFadeAnimationThrow (Variables|Target|GetPlrRef)))
      (:then_4
        (Physics|SetPhysicsLinearVelocity (Variables|Default|GetGasTank) (* (Math|Vector|GetForwardVector (Variables|/Game/Assets/Blueprint/Player/BP_Player.BP_Player_C|GetFPSCamera Plr)) 1.2e+03) false "None")))
    (else
      (CallFunction|ForceDrop Plr))))

(event EventShowCustomDepth
  (params (IsActive :type Boolean))
  ;[0.4491 1 0.2395] Set Post process
  (Rendering|SetRenderCustomDepth (Variables|Default|GetGasTank) IsActive))

(event EventDropObject
  (params (Plr :type BP%20Player%20Object%20Reference))
  ;[0.001821 0.04971 0.2462] Drop BPI
  (Variables|Target|SetPlrRef Plr)
  (Variables|Target|SetIsPickup? false)
  (Default|SetActorAttachGrab (Variables|Target|GetPlrRef))
  (Default|SetIsObjectPickup (Variables|Target|GetPlrRef) false)
  (Utilities|FlowControl|Sequence
    (:then_0
      (Actor|Tick|SetActorTickEnabled false))
    (:then_1
      (SETTER|SetCollisions "QueryAndPhysics")
      (SETTER|SetChannels "ECC_WorldDynamic")
      (SETTER|SetPhysics true))
    (:then_2
      (Utilities|Time|SetTimerbyEvent (EventDispatchers|CreateEvent :!event Custom|AutoResetCollision) 0.005)
      (Default|SettoCurrentWeapons (Variables|Target|GetPlrRef))
      (Default|SetEffectGrabObject (Variables|Target|GetPlrRef) true)
      (Default|SetColorPostLine (Variables|Target|GetPlrRef) false))))

(event EventGrabObject
  (params (Plr :type BP%20Player%20Object%20Reference))
  ;[0.2271 0.3215 1] Grab BPI
  (bind _output_get (Variables|Target|SetPlrRef Plr))
  (Variables|target|SetComponentToTarget (Variables|/Game/Assets/Blueprint/Player/BP_Player.BP_Player_C|GetObjectPos _output_get))
  (Default|SetActorAttachGrab (Variables|Target|GetPlrRef) self)
  (Utilities|FlowControl|Sequence
    (:then_0
      (Variables|Target|SetIsPickup? true)
      (Variables|Target|SetIsGrabbed true)
      (Default|SetWeaponsType (Variables|Target|GetPlrRef) "NewEnumerator2")
      (Default|DisableLogicWeapons (Variables|Target|GetPlrRef))
      (Default|SetEffectGrabObject (Variables|Target|GetPlrRef) false))
    (:then_1
      (SETTER|SetPhysics false))
    (:then_2
      (SETTER|SetCollisions "PhysicsOnly")
      (SETTER|SetCollisionsChannels "ECC_Pawn" "ECR_Ignore")
      (SETTER|SetChannels "ECC_PhysicsBody"))
    (:then_3
      (Actor|Tick|SetActorTickEnabled true))))

(event EventTick
  (params (DeltaSeconds :type Float%20%28single-precision%29))
  ;[0.07292 0.001139 0.001139] TICK
  (Variables|Tick|SetDelta%20Seconds DeltaSeconds)
  (Tick|FollowObject))

(event Game|Damage|EventAnyDamage
  (params (Damage :type Float%20%28single-precision%29) (DamageType :type Damage%20Type%20Object%20Reference) (InstigatedBy :type Controller%20Object%20Reference) (DamageCauser :type Actor%20Object%20Reference))
  ;[0.04667 0.2086 0.15] Get Any Damage
  (Utilities|FlowControl|DoOnce false
    (:Completed
      (AUTO|DestroyActorbyHit))))

(event EventBeginPlay)

(fn ConstructionScript
  (Components|StaticMesh|SetStaticMesh (Variables|Default|GetGasTank) (Utilities|Select :Index (Variables|ProfileTank|GetGasType) :NewEnumerator0 "/Game/Megascans/3D_Assets/Gas/Rusty_Gas_Tank_udmkdejqx/S_Rusty_Gas_Tank_udmkdejqx_lod3.S_Rusty_Gas_Tank_udmkdejqx_lod3" :NewEnumerator1 "/Game/Megascans/3D_Assets/Gas/Rusty_Gas_Tank_tl1rbitfa/S_Rusty_Gas_Tank_tl1rbitfa_lod3.S_Rusty_Gas_Tank_tl1rbitfa_lod3" :NewEnumerator2 "/Game/Megascans/3D_Assets/Gas/Rusty_Gas_Tank_udmkdejqx/S_Rusty_Gas_Tank_udmkdejqx_lod3.S_Rusty_Gas_Tank_udmkdejqx_lod3" :NewEnumerator3 "/Game/Megascans/3D_Assets/Gas/Rusty_Gas_Tank_udmkdejqx/S_Rusty_Gas_Tank_udmkdejqx_lod3.S_Rusty_Gas_Tank_udmkdejqx_lod3" :NewEnumerator4 "/Game/Megascans/3D_Assets/Gas/Rusty_Gas_Tank_tl1rbitfa/S_Rusty_Gas_Tank_tl1rbitfa_lod3.S_Rusty_Gas_Tank_tl1rbitfa_lod3"))
  (Rendering|Material|SetMaterial (Variables|Default|GetGasTank) 0 (Utilities|Select :Index (Variables|ProfileTank|GetGasType) :NewEnumerator0 "/Game/Megascans/3D_Assets/Gas/Rusty_Gas_Tank_udmkdejqx/MI_Rusty_Gas_Tank_udmkdejqx_EXPLOSIVE.MI_Rusty_Gas_Tank_udmkdejqx_EXPLOSIVE" :NewEnumerator1 "/Game/Megascans/3D_Assets/Gas/Rusty_Gas_Tank_tl1rbitfa/MI_Rusty_Gas_Tank_tl1rbitfa_2K1_Flammable.MI_Rusty_Gas_Tank_tl1rbitfa_2K1_Flammable" :NewEnumerator2 "/Game/Megascans/3D_Assets/Gas/Rusty_Gas_Tank_udmkdejqx/MI_Rusty_Gas_Tank_udmkdejqx_Smoke.MI_Rusty_Gas_Tank_udmkdejqx_Smoke" :NewEnumerator3 "/Game/Megascans/3D_Assets/Gas/Rusty_Gas_Tank_udmkdejqx/MI_Rusty_Gas_Tank_udmkdejqx_TOXIC.MI_Rusty_Gas_Tank_udmkdejqx_TOXIC" :NewEnumerator4 "/Game/Megascans/3D_Assets/Gas/Rusty_Gas_Tank_tl1rbitfa/MI_Rusty_Gas_Tank_tl1rbitfa_2K1_Goo.MI_Rusty_Gas_Tank_tl1rbitfa_2K1_Goo")))

(fn FollowObject
  (bind _componenttotarget (Variables|target|GetComponentToTarget))
  (Variables|Target|GetPlrRef
    (:then
      (Variables|target|GetComponentToTarget
        (:then
          (if (Variables|Target|GetIsPickup?)
            (LocalVariables|SetCompLoc (Transformation|GetWorldLocation _componenttotarget))
            (LocalVariables|SetCompRot (Transformation|GetWorldRotation _componenttotarget))
            (Transformation|SetActorLocation (Math|Interpolation|VInterpTo (Transformation|GetActorLocation) (LocalVariables|GetCompLoc) (Variables|Tick|GetDelta%20Seconds) 4e+01) false false)
            (Transformation|SetActorRotation (Math|Interpolation|RInterpTo (Transformation|GetActorRotation) (LocalVariables|GetCompRot) (Variables|Tick|GetDelta%20Seconds) 2e+01))))
        (:else)))
    (:else)))

(fn SetCollisions
  (params (NewType :type ECollisionEnabled%20Enum :default "NoCollision"))
  (Collision|SetCollisionEnabled (Variables|Default|GetGasTank) NewType))

(fn SetPhysics
  (params (bSimulate :type Boolean))
  (Physics|SetSimulatePhysics (Variables|Default|GetGasTank) bSimulate))

(fn SetCollisionsChannels
  (params (Channel :type ECollisionChannel%20Enum :default "ECC_WorldStatic") (NewResponse :type ECollisionResponse%20Enum :default "ECR_Ignore"))
  (Collision|SetCollisionResponsetoChannel (Variables|Default|GetGasTank) Channel NewResponse))

(fn SetChannels
  (params (Channel :type ECollisionChannel%20Enum :default "ECC_WorldStatic"))
  (Collision|SetCollisionObjectType (Variables|Default|GetGasTank) Channel))

(fn GetVelocityActor
  (return (Math|Vector|VectorLength (Transformation|GetComponentVelocity (Variables|Default|GetGasTank)))))

(fn DestroyActorbyHit
  (Effects|SpawnEmitteratLocation (Utilities|GetEffecttoDestroy) (Transformation|GetActorLocation))
  (Game|SpawnActorfromClass (Utilities|Select :Index (Variables|ProfileTank|GetGasType) :NewEnumerator0 "/Game/Assets/Blueprint/Props/GasTank/BP_Explosive.BP_Explosive_C" :NewEnumerator1 0 :NewEnumerator2 0 :NewEnumerator3 0 :NewEnumerator4 "/Game/Assets/Blueprint/Props/GasTank/BP_GooMaster.BP_GooMaster_C") (Math|Transform|MakeTransform (Transformation|GetActorLocation) "0, 0, 0" "1.000000,1.000000,1.000000") "AlwaysSpawn" "MultiplyWithRoot" 0 0)
  (Actor|DestroyActor))

(fn CreateChaosDestruction
  (params (Spawn%20Transform%20Location :type Vector) (Size :type Float%20%28double-precision%29))
  (bind _returnvalue (Game|SpawnActorfromClass "/Game/Assets/Blueprint/Chaos/FS_MasterField_Custom.FS_MasterField_Custom_C" (Math|Transform|MakeTransform Spawn%20Transform%20Location "0, 0, 0" (Math|Vector|MakeVector Size Size Size)) "AlwaysSpawn" "MultiplyWithRoot" 0 0))
  (Actor|SetLifeSpan _returnvalue 3.0)
  (Variables|/Game/Assets/Blueprint/Chaos/FS_MasterField_Custom.FS_MasterField_Custom_C|SetActivationType _returnvalue "NewEnumerator4")
  (Variables|/Game/Assets/Blueprint/Chaos/FS_MasterField_Custom.FS_MasterField_Custom_C|SetFieldLifespan _returnvalue 0.1)
  (Variables|/Game/Assets/Blueprint/Chaos/FS_MasterField_Custom.FS_MasterField_Custom_C|SetRadial%20Magnitude _returnvalue 8e+02)
  (Default|CETrigger _returnvalue))