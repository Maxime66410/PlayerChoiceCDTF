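; BP_CatchMoney is a catch zone that pays the player money when a prop of one specific type enters its box.
; On overlap it checks the BP_PropMaster's type and applies massive damage to a match, then spawns two Niagara effects at its arrow component.
; After a short delay it calls AddMoney with a fixed reward on the BP_Player reference cached at BeginPlay.
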(event OnComponentBeginOverlap(Box)
  (params (OverlappedComponent :type Primitive%20Component%20Object%20Reference) (OtherActor :type Actor%20Object%20Reference) (OtherComp :type Primitive%20Component%20Object%20Reference) (OtherBodyIndex :type Integer) (bFromSweep :type Boolean) (SweepResult :type Hit%20Result%20Structure%20%28by%20ref%29))
  (bind _arrow (Variables|Default|GetArrow))
  (bind _returnvalue (Transformation|GetWorldLocation _arrow))
  (bind _returnvalue_2 (Transformation|GetWorldRotation _arrow))
  (bind _asbp_prop_master (Utilities|Casting|CastToBP_PropMaster OtherActor))
  (if (Utilities|Enum|Equal(Enum) (Variables|/Game/Assets/Blueprint/Props/BP_PropMaster.BP_PropMaster_C|GetPropType _asbp_prop_master) "NewEnumerator8")
    (Game|Damage|ApplyDamage _asbp_prop_master 9999999999.0 0 self)
    (Niagara|SpawnSystematLocation "/Game/Assets/Effects/NS_CatchPropsEffect.NS_CatchPropsEffect" _returnvalue _returnvalue_2)
    (Niagara|SpawnSystematLocation "/Game/Assets/Effects/NS_GetFlag.NS_GetFlag" _returnvalue _returnvalue_2 "2.000000,2.000000,2.000000")
    (Utilities|FlowControl|Delay 0.2)
    (Default|AddMoney (Variables|Default|GetREF_Player) 350)))

(event EventBeginPlay
  (CallFunction|GetPlayer))

(fn ConstructionScript)

(fn GetPlayer
  (bind _returnvalue (Actor|GetActorOfClass "/Game/Assets/Blueprint/Player/BP_Player.BP_Player_C"))
  (Variables|Default|SetREF_Player _returnvalue))