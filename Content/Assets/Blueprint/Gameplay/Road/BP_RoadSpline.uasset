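; BP_RoadSpline is a road actor that builds its geometry from spline mesh segments laid along a spline.
; The construction script steps along the spline in SizeMesh increments, shortening the last segment to end exactly at the spline's length.
; Each segment takes local-space positions and tangents from the spline, with tangents clamped to half SizeMesh.
; The event graph has no active logic.
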(event EventBeginPlay)

(event Collision|EventActorBeginOverlap
  (params (OtherActor :type Actor%20Object%20Reference)))

(event EventTick
  (params (DeltaSeconds :type Float%20%28single-precision%29)))

(fn ConstructionScript
  (bind _sizemesh (Variables|Default|GetSizeMesh))
  (bind _returnvalue (/ _sizemesh 2.0))
  (LocalVariables|SetSplineLength (Spline|GetSplineLength (Variables|Default|GetSpline)))
  (LocalVariables|SetActualDistance 0.0)
  (while (< (LocalVariables|GetActualDistance) (LocalVariables|GetSplineLength))
    (LocalVariables|SetStartLocation (Spline|GetLocationatDistanceAlongSpline (Variables|Default|GetSpline) (LocalVariables|GetActualDistance) "Local"))
    (LocalVariables|SetStartTangent (Spline|GetTangentatDistanceAlongSpline (Variables|Default|GetSpline) (LocalVariables|GetActualDistance) "Local"))
    (LocalVariables|SetActualDistance (select (> (+ (LocalVariables|GetActualDistance) (Variables|Default|GetSizeMesh)) (LocalVariables|GetSplineLength)) (LocalVariables|GetSplineLength) (+ (LocalVariables|GetActualDistance) (Variables|Default|GetSizeMesh))))
    (LocalVariables|SetEndLocation (Spline|GetLocationatDistanceAlongSpline (Variables|Default|GetSpline) (LocalVariables|GetActualDistance) "Local"))
    (LocalVariables|SetEndTangent (Spline|GetTangentatDistanceAlongSpline (Variables|Default|GetSpline) (LocalVariables|GetActualDistance) "Local"))
    (bind _returnvalue_2 (AddComponent|AddSplineMeshComponent false))
    (SplineMesh|SetStartandEnd _returnvalue_2 (LocalVariables|GetStartLocation) (Math|Vector|ClampVectorSize (LocalVariables|GetStartTangent) 0.0 _returnvalue) (LocalVariables|GetEndLocation) (Math|Vector|ClampVectorSize (LocalVariables|GetEndTangent) 0.0 _returnvalue) true :!class /Script/Engine.SplineMeshComponent)))