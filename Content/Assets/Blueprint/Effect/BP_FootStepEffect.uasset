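; Footprint decal actor whose material matches a surface type: mud, snow or sand.
; The construction script applies the material selected by TypeDecal, and ChangeDecalType updates the type and reapplies the material at runtime.
; On BeginPlay it randomly negates the actor's Y scale, mirroring some prints for variation.
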(event Custom|ChangeDecalType
  (params (TypeDecal :type EFootStepEffect%20Enum :default "NewEnumerator0"))
  (Variables|Default|SetTypeDecal TypeDecal)
  (Rendering|Components|Decal|SetDecalMaterial (Variables|Decal|GetDecal) (Utilities|Select :Index (Variables|Default|GetTypeDecal) :NewEnumerator0 "/Game/Megascans/Decals/Sand_Footprint_ukftbe2cw/MI_Sand_Footprint_ukftbe2cw_2K.MI_Sand_Footprint_ukftbe2cw_2K" :NewEnumerator1 "/Game/Megascans/Decals/Sand_Footprint_ukftbe2cw/MI_Sand_Footprint_ukftbe2cw_Snow.MI_Sand_Footprint_ukftbe2cw_Snow" :NewEnumerator2 "/Game/Megascans/Decals/Sand_Footprint_ukftbe2cw/MI_Sand_Footprint_ukftbe2cw_Sands.MI_Sand_Footprint_ukftbe2cw_Sands")))

(event EventBeginPlay
  (bind _returnvalue (Transformation|GetActorScale3D))
  (Transformation|SetActorScale3D (Math|Vector|MakeVector (.x _returnvalue) (select (Math|Random|RandomBool) (* (.y _returnvalue) -1.0) (.y _returnvalue)) (.z _returnvalue))))

(fn ConstructionScript
  (Rendering|Components|Decal|SetDecalMaterial (Variables|Decal|GetDecal) (Utilities|Select :Index (Variables|Default|GetTypeDecal) :NewEnumerator0 "/Game/Megascans/Decals/Sand_Footprint_ukftbe2cw/MI_Sand_Footprint_ukftbe2cw_2K.MI_Sand_Footprint_ukftbe2cw_2K" :NewEnumerator1 "/Game/Megascans/Decals/Sand_Footprint_ukftbe2cw/MI_Sand_Footprint_ukftbe2cw_Snow.MI_Sand_Footprint_ukftbe2cw_Snow" :NewEnumerator2 "/Game/Megascans/Decals/Sand_Footprint_ukftbe2cw/MI_Sand_Footprint_ukftbe2cw_Sands.MI_Sand_Footprint_ukftbe2cw_Sands")))