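; Interactive garage door that the player toggles open and closed by pressing E.
; BeginPlay and entering the Trigger enable input and open a gate, with overlap also printing a prompt; leaving the Trigger disables both.
; E passes through the gate to play the skeletal mesh's open or close animation based on DoorIsClosed.
; A temporary boolean blocks retriggering until a fixed delay ends and flips the state.
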(event OnComponentEndOverlap(Trigger)
  (params (OverlappedComponent :type Primitive%20Component%20Object%20Reference) (OtherActor :type Actor%20Object%20Reference) (OtherComp :type Primitive%20Component%20Object%20Reference) (OtherBodyIndex :type Integer))
  (Input|DisableInput (Game|GetPlayerController 0))
  (Utilities|FlowControl|Gate true) ; enters at Close
)

(event OnComponentBeginOverlap(Trigger)
  (params (OverlappedComponent :type Primitive%20Component%20Object%20Reference) (OtherActor :type Actor%20Object%20Reference) (OtherComp :type Primitive%20Component%20Object%20Reference) (OtherBodyIndex :type Integer) (bFromSweep :type Boolean) (SweepResult :type Hit%20Result%20Structure%20%28by%20ref%29))
  (Development|PrintText "Press E" true false "(R=1.000000,G=1.000000,B=1.000000,A=1.000000)" 1.0)
  (Input|EnableInput (Game|GetPlayerController 0))
  (Utilities|FlowControl|Gate true) ; enters at Open
)

(event EventBeginPlay
  (Input|EnableInput (Game|GetPlayerController 0))
  (Utilities|FlowControl|Gate true) ; enters at Open
)

(event Input|KeyboardEvents|E
  (params (Key :type Key%20Structure))
  (:Pressed
    (Utilities|FlowControl|Gate true
      (:Exit
        (if (Math|Boolean|Equal(Boolean) (Variables|Default|Gettemperal_bln) false)
          (if (Math|Boolean|Equal(Boolean) (Variables|Default|GetDoor_Is_Closed) true)
            (Variables|Default|Settemperal_bln true)
            (Components|Animation|PlayAnimation (Variables|Default|GetSK_Door_Garage_A) "/Game/Assets/Models/ModularHouses/Animation/SK_Door_Garage_A_Open_Anim.SK_Door_Garage_A_Open_Anim" false)
            (Utilities|FlowControl|Delay 6.67)
            (Variables|Default|SetDoor_Is_Closed false)
            (Variables|Default|Settemperal_bln false)
            (else
              (Variables|Default|Settemperal_bln true)
              (Components|Animation|PlayAnimation (Variables|Default|GetSK_Door_Garage_A) "/Game/Assets/Models/ModularHouses/Animation/SK_Door_Garage_A_Closed_Anim.SK_Door_Garage_A_Closed_Anim" false)
              (Utilities|FlowControl|Delay 6.67)
              (Variables|Default|SetDoor_Is_Closed true)
              (Variables|Default|Settemperal_bln false))))))))

(fn ConstructionScript)